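; BP_BurnableTreeTrunk is a tree trunk actor the player can burn away with an equipped torch.
; On BeginPlay it caches the first BP_Player in the level.
; Overlapping FlameDetection with the torch equipped sets the burn flags and "F - Burn" prompt on the player, and leaving clears them.
; The Burn_Tree event rechecks only the equipped torch, then destroys the trunk immediately.
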(event OnComponentBeginOverlap(FlameDetection)
  (params (OverlappedComponent :type Primitive%20Component%20Object%20Reference) (OtherActor :type Actor%20Object%20Reference) (OtherComp :type Primitive%20Component%20Object%20Reference) (OtherBodyIndex :type Integer) (bFromSweep :type Boolean) (SweepResult :type Hit%20Result%20Structure%20%28by%20ref%29))
  (bind _player (Variables|Default|GetPlayer))
  (if (== (Variables|/Game/Blueprints/BP_Player.BP_Player_C|GetisEquipped? (Variables|Default|GetPlayer)) 3)
    (Variables|Default|SetCan%20Burn? true)
    (Variables|/Game/Blueprints/BP_Player.BP_Player_C|SetCurrentInteractText _player "F - Burn")
    (Variables|/Game/Blueprints/BP_Player.BP_Player_C|SetCanBurn? _player true)))

(event OnComponentEndOverlap(FlameDetection)
  (params (OverlappedComponent :type Primitive%20Component%20Object%20Reference) (OtherActor :type Actor%20Object%20Reference) (OtherComp :type Primitive%20Component%20Object%20Reference) (OtherBodyIndex :type Integer))
  (bind _player (Variables|Default|GetPlayer))
  (Variables|Default|SetCan%20Burn? false)
  (Variables|/Game/Blueprints/BP_Player.BP_Player_C|SetCurrentInteractText _player "")
  (Variables|/Game/Blueprints/BP_Player.BP_Player_C|SetCanBurn? _player false))

(event Custom|Burn_Tree
  (if (== (Variables|/Game/Blueprints/BP_Player.BP_Player_C|GetisEquipped? (Variables|Default|GetPlayer)) 3)
    (Actor|DestroyActor)))

(event Collision|EventActorBeginOverlap
  (params (OtherActor :type Actor%20Object%20Reference)))

(event EventBeginPlay
  (bind _outactors (Actor|GetAllActorsOfClass "/Game/Blueprints/BP_Player.BP_Player_C"))
  (Variables|Default|SetPlayer (Utilities|Array|Get(acopy) _outactors)))

(fn ConstructionScript)