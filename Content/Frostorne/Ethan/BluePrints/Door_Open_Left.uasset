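; Left door actor that swings open for a key-holding player or an approaching guard enemy.
; Trigger overlap checks the player for the required key, enabling input and showing an interact prompt, or a key-needed message; exit clears both.
; Interact input or a guard overlap plays a timeline that lerps root yaw to a quarter turn.
; The graph has no closing logic.
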(event OnComponentEndOverlap(TriggerBox)
  (params (OverlappedComponent :type Primitive%20Component%20Object%20Reference) (OtherActor :type Actor%20Object%20Reference) (OtherComp :type Primitive%20Component%20Object%20Reference) (OtherBodyIndex :type Integer))
  (bind _asbp_player (Utilities|Casting|CastToBP_Player OtherActor)
    (:then
      (Input|DisableInput (Game|GetPlayerController 0))
      (Variables|/Game/Blueprints/BP_Player.BP_Player_C|SetCurrentInteractText _asbp_player ""))
    (:CastFailed
      (Utilities|Casting|CastToBP_GuardEnemy OtherActor))))

(event OnComponentBeginOverlap(TriggerBox)
  (params (OverlappedComponent :type Primitive%20Component%20Object%20Reference) (OtherActor :type Actor%20Object%20Reference) (OtherComp :type Primitive%20Component%20Object%20Reference) (OtherBodyIndex :type Integer) (bFromSweep :type Boolean) (SweepResult :type Hit%20Result%20Structure%20%28by%20ref%29))
  (bind _asbp_player (Utilities|Casting|CastToBP_Player OtherActor)
    (:then
      (bind _has_key (Default|HasKey _asbp_player (Variables|Default|GetRequiredKey?)))
      (if _has_key
        (Input|EnableInput (Game|GetPlayerController 0))
        (Variables|/Game/Blueprints/BP_Player.BP_Player_C|SetCurrentInteractText _asbp_player "E - Open Left Door")
        (else
          (Variables|/Game/Blueprints/BP_Player.BP_Player_C|SetCurrentInteractText _asbp_player "You Need A Key ?"))))
    (:CastFailed
      (Utilities|Casting|CastToBP_GuardEnemy OtherActor)
      (bind _doorfloat (Timeline|OpenDoor1 Play)
        (:Update
          (Transformation|SetRelativeRotation (Variables|Default|GetRoot) (Math|Rotator|MakeRotator 0.0 0.0 (Math|Float|Lerp 0.0 -9e+01 _doorfloat)) false false))))))

(event Input|ActionEvents|InputActionInteract
  (params (Key :type Key%20Structure :default "None"))
  (:Pressed
    (bind _doorfloat (Timeline|OpenDoor1 Play)
      (:Update
        (Transformation|SetRelativeRotation (Variables|Default|GetRoot) (Math|Rotator|MakeRotator 0.0 0.0 (Math|Float|Lerp 0.0 -9e+01 _doorfloat)) false false)))))

(fn ConstructionScript)